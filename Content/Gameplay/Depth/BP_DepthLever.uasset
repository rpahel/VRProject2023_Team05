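; VR grabbable lever that broadcasts activation and deactivation events and shows its state on a diode material.
; While held, Tick projects the lever-to-motion-controller vector onto the plane normal to the actor's forward vector, then uses an atan2 difference against actor up for clamped roll.
; Reaching a margin below maximum angle activates it; leaving that zone deactivates it.
; Release snaps it back to minimum angle and fires deactivation.
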(event OnGrabbed(GrabComponent)
  (bind _grabcomponent (Variables|Default|GetGrabComponent))
  (Utilities|IsValid _grabcomponent
    (:Is%20Valid
      (bind _motioncontroller (Default|GetMotionControllerRef _grabcomponent))
      (Variables|PasTouche|SetMotion%20Controller _motioncontroller))))

(event OnDropped(GrabComponent)
  (Variables|PasTouche|SetMotion%20Controller 0)
  (Variables|PasTouche|SetIsActivated false)
  (Default|CallOnLeverDeactivated)
  (Transformation|SetRelativeRotation (Variables|Default|GetLeverActuator_Root) (Math|Rotator|MakeRotator (Variables|Important|GetLeverAngleMin) 0.0 0.0) false false))

(event Custom|Event%20LeverActivated
  (bind _diode (Variables|Default|GetDiode))
  (Utilities|IsValid _diode
    (:Is%20Valid
      (Rendering|Material|SetMaterial _diode 0 (Variables|PasImportant|GetDiodeLitMaterial)))))

(event Custom|Event%20LeverDeactivated
  (bind _diode (Variables|Default|GetDiode))
  (Utilities|IsValid _diode
    (:Is%20Valid
      (Rendering|Material|SetMaterial _diode 0 (Variables|PasImportant|GetDiodeUnlitMaterial)))))

(event EventTick
  (params (DeltaSeconds :type Float%20%28single-precision%29))
  (CallFunction|UpdateLeverRotation))

(event EventBeginPlay
  (bind _leveractuator_root (Variables|Default|GetLeverActuator_Root))
  (Utilities|IsValid _leveractuator_root
    (:Is%20Valid
      (Transformation|SetRelativeRotation _leveractuator_root (Math|Rotator|MakeRotator (Variables|Important|GetLeverAngleMin) 0.0 0.0) false false)
      (EventDispatchers|BindEventtoOnLeverActivated (delegate Custom|Event%20LeverActivated))
      (EventDispatchers|BindEventtoOnLeverDeactivated (delegate Custom|Event%20LeverDeactivated)))))

(fn ConstructionScript)

(fn UpdateLeverRotation
  (bind _returnvalue (Transformation|GetActorForwardVector))
  (bind _returnvalue_2 (Transformation|GetActorUpVector))
  (bind _returnvalue_3 (Transformation|GetActorLocation))
  (bind _motion_controller (Variables|PasTouche|GetMotion%20Controller))
  (bind _leveranglemin (Variables|Important|GetLeverAngleMin))
  (bind _leveranglemax (Variables|Important|GetLeverAngleMax))
  (bind _returnvalue_4 (Transformation|GetWorldLocation _motion_controller))
  (bind _returnvalue_5 (Class|KismetMathLibrary|DegAtan2 (.z _returnvalue_2) (.y _returnvalue_2)))
  (bind _returnvalue_6 (- _returnvalue_4 _returnvalue_3))
  (bind _returnvalue_7 (Math|Vector|ProjectVectorontoPlane _returnvalue_6 _returnvalue))
  (bind _returnvalue_8 (Math|Vector|Normalize _returnvalue_7))
  (bind _returnvalue_9 (Class|KismetMathLibrary|DegAtan2 (.z _returnvalue_8) (.y _returnvalue_8)))
  (bind _returnvalue_10 (- _returnvalue_5 _returnvalue_9))
  (bind _returnvalue_11 (Math|Float|Clamp(Float) _returnvalue_10 _leveranglemin _leveranglemax))
  (Utilities|IsValid _motion_controller
    (:Is%20Valid
      (Transformation|SetRelativeRotation (Variables|Default|GetLeverActuator_Root) (Math|Rotator|MakeRotator _returnvalue_11 0.0 0.0) false false)
      (if (>= _returnvalue_11 (- (Variables|Important|GetLeverAngleMax) (Variables|Important|GetDeltaLeverActivation)))
        (if (not (Variables|PasTouche|GetIsActivated))
          (Variables|PasTouche|SetIsActivated true)
          (Default|CallOnLeverActivated))
        (elif (Variables|PasTouche|GetIsActivated)
          (Variables|PasTouche|SetIsActivated false)
          (Default|CallOnLeverDeactivated))))))