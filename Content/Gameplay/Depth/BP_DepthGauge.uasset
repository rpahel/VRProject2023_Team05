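; Depth gauge that, while plugged into the electric box and activated by its lever, raises depth toward the surface, printing a placeholder victory at zero.
; Depth changes feed a screen widget, whose level-reached event starts a decompression timer.
; Ascending during that timer fires respected or ignored dispatchers based on a grace delay.
; Cable state toggles the diode and screen, while audio triggers drive gear and sonar sounds.
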(event Custom|OnCablePlugged
  (params (FemalePlugIndex :type Integer))
  ;[1 1 1] Bind plugged
  (CallFunction|CablePlugged FemalePlugIndex))

(event Custom|OnCableUnplugged
  (params (FemalePlugIndex :type Integer))
  ;[1 1 1] Bind Unplugged
  (Utilities|FlowControl|Sequence
    (:then_0
      (CallFunction|CableUnplugged FemalePlugIndex))))

(event Custom|DepthChangedEvent
  (params (NewDepth :type Float%20%28double-precision%29))
  (bind _depthgaugescreen (Variables|DoNotTouch|GetDepthGaugeScreen))
  (Utilities|IsValid _depthgaugescreen
    (:Is%20Valid
      (Default|UpdateDepth _depthgaugescreen NewDepth))))

(event Custom|Event%20DepthLevelReached
  (bind _returnvalue (Utilities|Time|SetTimerbyEvent (delegate Custom|Event%20DecompressionFinished) (Variables|Dependences|GetDecompressionWaitTime)))
  (Variables|Default|SetDecompressionTimerHandle _returnvalue)
  (Class|AudioParameterControllerInterface|SetTriggerParameter (Variables|Default|GetMS_CP) "FastSonar"))

(event Custom|Event%20DecompressionFinished
  (Utilities|Time|ClearandInvalidateTimerbyHandle (Variables|Default|GetDecompressionTimerHandle))
  (Default|CallOnDecompressionIgnoredStopped)
  (Class|AudioParameterControllerInterface|SetTriggerParameter (Variables|Default|GetMS_CP) "NormalSonar"))

(event Custom|Event%20LeverActivated
  (Variables|Donottouch|SetIsActivated true))

(event Custom|Event%20LeverDeactivated
  (bind _decompressiontimerhandle (Variables|Default|GetDecompressionTimerHandle))
  (Variables|Donottouch|SetIsActivated false)
  ;[1 1 1] Check voir si on est en décompression
  (if (and (Utilities|Time|IsValidTimerHandle _decompressiontimerhandle) (Utilities|Time|IsTimerActivebyHandle _decompressiontimerhandle))
    (Default|CallOnDecompressionIgnoredStopped)))

(event EventBeginPlay
  (bind _electricbox (Variables|Dependences|GetElectricBox))
  (bind _depthgaugewidget (Variables|Default|GetDepthGaugeWidget))
  (bind _depthlever (Variables|Dependences|GetDepthLever))
  (Utilities|FlowControl|Sequence
    (:then_0
      (Audio|Components|Audio|Play (Variables|Default|GetMS_CP) 0.0))
    (:then_1
      (Variables|Donottouch|SetIsPlugged false)
      (Variables|DoNotTouch|SetCurrentDepth (Variables|Dependences|GetStartingDepth))
      (Utilities|IsValid _electricbox
        (:Is%20Valid
          ;[1 1 1] Bind plugged
          (EventDispatchers|BindEventtoOnCablePlugged _electricbox (delegate Custom|OnCablePlugged))
          ;[1 1 1] Bind Unplugged
          (EventDispatchers|BindEventtoOnCableUnplugged _electricbox (delegate Custom|OnCableUnplugged))
          ;[1 1 1] Set DepthGaugeScreen
          (Utilities|IsValid _depthgaugewidget
            (:Is%20Valid
              (bind _asw_depth_gauge_screen (Utilities|Casting|CastToW_DepthGaugeScreen (UserInterface|GetWidget _depthgaugewidget)))
              (bind _output_get (Variables|DoNotTouch|SetDepthGaugeScreen _asw_depth_gauge_screen))
              (Default|SetUp _output_get (Variables|Dependences|GetDecompressionWaitTime) (Variables|Dependences|GetStartingDepth) (Variables|Dependences|GetNbOfDepthLevels))
              (EventDispatchers|BindEventtoOnDepthLevelReached (Variables|DoNotTouch|GetDepthGaugeScreen) (delegate Custom|Event%20DepthLevelReached))
              ;[1 1 1] Autres
              (EventDispatchers|BindEventtoOnDepthChanged (delegate Custom|DepthChangedEvent))
              (bind _output_get_2 (Variables|DoNotTouch|SetCurrentDepth (Variables|Dependences|GetStartingDepth)))
              (Default|CallOnDepthChanged _output_get_2)
              (CallFunction|CableUnplugged (Variables|Dependences|GetFemalePlugIndex))
              ;[1 1 1] Bind au levier
              (Utilities|IsValid _depthlever
                (:Is%20Valid
                  (EventDispatchers|BindEventtoOnLeverActivated _depthlever (delegate Custom|Event%20LeverActivated))
                  (EventDispatchers|BindEventtoOnLeverDeactivated _depthlever (delegate Custom|Event%20LeverDeactivated)))))))))))

(event EventTick
  (params (DeltaSeconds :type Float%20%28single-precision%29))
  (bind _decompressiontimerhandle (Variables|Default|GetDecompressionTimerHandle))
  (bind _ms_cp (Variables|Default|GetMS_CP))
  (Utilities|FlowControl|Sequence
    (:then_0
      (if (and (Variables|Donottouch|GetIsPlugged) (Variables|Donottouch|GetIsActivated))
        (if (>= (Variables|DoNotTouch|GetCurrentDepth) 0.0)
          (Development|PrintString "Victory !" true true "(R=0.000000,G=0.660000,B=1.000000,A=1.000000)" 0.0)
          (else
            ;[1 1 1] Update de la profondeur
            (bind _output_get (Variables|DoNotTouch|SetCurrentDepth (|({DBE92AA1-49FA-665A-B920-CF8C05DE56BE}+((AbsStartingDepth/{6E48C658-475C-8D76-3632-80B87836E7FD})*DeltaSeconds)) DeltaSeconds (Math|Float|Absolute(Float) (Variables|Dependences|GetStartingDepth)))))
            (Default|CallOnDepthChanged _output_get)
            ;[1 1 1] Check voir si on est en décompression
            (if (and (Utilities|Time|IsValidTimerHandle _decompressiontimerhandle) (Utilities|Time|IsTimerActivebyHandle _decompressiontimerhandle))
              ;[1 1 1] Délai de grâce
              (if (>= (Class|KismetSystemLibrary|GetTimerElapsedTimeHandle _decompressiontimerhandle) (Variables|Dependences|GetDelaiDeGrace))
                (Default|CallOnDecompressionIgnored)
                (else
                  (Default|CallOnDecompressionRespected))))))))
    (:then_1
      (if (Variables|Donottouch|GetIsPlugged)
        (Utilities|FlowControl|Sequence
          (:then_0
            (if (Variables|Donottouch|GetIsActivated)
              (Utilities|FlowControl|DoOnce false :!label _label
                (:Completed
                  (Class|AudioParameterControllerInterface|SetTriggerParameter (Variables|Default|GetMS_CP) "GearOn")
                  (goto _label_2 Reset)))
              (else
                (Utilities|FlowControl|DoOnce false :!label _label_2
                  (:Completed
                    (Class|AudioParameterControllerInterface|SetTriggerParameter (Variables|Default|GetMS_CP) "GearOff")
                    (goto _label Reset))))))
          (:then_1
            (Utilities|FlowControl|DoOnce false :!label _label_3
              (:Completed
                (Class|AudioParameterControllerInterface|SetTriggerParameter _ms_cp "NormalSonar")
                (Class|AudioParameterControllerInterface|SetTriggerParameter _ms_cp "PlayCP")))))
        (else
          (Utilities|FlowControl|Sequence
            (:then_0
              (Class|AudioParameterControllerInterface|SetTriggerParameter (Variables|Default|GetMS_CP) "StopCP")
              (goto _label_3 Reset))))))))

(fn ConstructionScript)

(fn CablePlugged
  (params (PlugIndex :type Integer))
  (bind _diode_sm (Variables|Default|GetDiode_SM))
  (bind _depthgaugescreen (Variables|DoNotTouch|GetDepthGaugeScreen))
  (if (== (Variables|Dependences|GetFemalePlugIndex) PlugIndex)
    (Variables|Donottouch|SetIsPlugged true)
    ;[1 1 1] Diode
    (Utilities|IsValid _diode_sm
      (:Is%20Valid
        (Rendering|Material|SetMaterial _diode_sm 0 (Variables|Appearance|GetLitDiodeMaterial))
        ;[1 1 1] Turn Screen On
        (Utilities|IsValid _depthgaugescreen
          (:Is%20Valid
            (Default|TurnonorOff _depthgaugescreen true)))))))

(fn CableUnplugged
  (params (PlugIndex :type Integer))
  (bind _diode_sm (Variables|Default|GetDiode_SM))
  (bind _depthgaugescreen (Variables|DoNotTouch|GetDepthGaugeScreen))
  (if (== (Variables|Dependences|GetFemalePlugIndex) PlugIndex)
    (Variables|Donottouch|SetIsPlugged false)
    ;[1 1 1] Diode
    (Utilities|IsValid _diode_sm
      (:Is%20Valid
        (Rendering|Material|SetMaterial _diode_sm 0 (Variables|Appearance|GetUnlitDiodeMaterial))
        ;[1 1 1] Turn Screen Off
        (Utilities|IsValid _depthgaugescreen
          (:Is%20Valid
            (Default|TurnonorOff _depthgaugescreen false)))))))

(fn TestON
  (CallFunction|CablePlugged (Variables|Dependences|GetFemalePlugIndex)))

(fn TestOFF
  (CallFunction|CableUnplugged (Variables|Dependences|GetFemalePlugIndex)))

(fn TestACTIVATE
  (Utilities|IsValid (Variables|Dependences|GetDepthLever)
    (:Is%20Not%20Valid
      (Variables|Donottouch|SetIsActivated true))))

(fn TestDEACTIVATE
  (bind _decompressiontimerhandle (Variables|Default|GetDecompressionTimerHandle))
  (Utilities|IsValid (Variables|Dependences|GetDepthLever)
    (:Is%20Not%20Valid
      (Variables|Donottouch|SetIsActivated false)
      ;[1 1 1] Check voir si on est en décompression
      (if (and (Utilities|Time|IsValidTimerHandle _decompressiontimerhandle) (Utilities|Time|IsTimerActivebyHandle _decompressiontimerhandle))
        (Default|CallOnDecompressionIgnoredStopped)))))