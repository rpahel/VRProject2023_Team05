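; VR water-level valve that the player grabs and turns to shut off the water temporarily.
; Tick rotates the mesh toward the held motion controller, calling DesactivateWater and locking once roll passes a threshold.
; A bound delayed reset uses a timeline to rotate it back, calls ReactivateWater and re-enables it after a cooldown.
; MSValve supplies triggered audio, and a test event simulates activation without grabbing.
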(event OnGrabbed(GrabComponent)
  (bind _grabcomponent (Variables|Default|GetGrabComponent))
  (Utilities|IsValid _grabcomponent
    (:Is%20Valid
      (bind _motioncontroller (Default|GetMotionControllerRef _grabcomponent))
      (Variables|Default|SetMotion%20Controller _motioncontroller))))

(event OnDropped(GrabComponent)
  (Variables|Default|SetMotion%20Controller 0))

(event Custom|LaunchDelay
  (bind _sm_valve_01 (Variables|Default|GetSM_Valve_01))
  (bind _returnvalue (Transformation|GetWorldRotation _sm_valve_01))
  ;[1 1 1] Reset
  (Utilities|FlowControl|RetriggerableDelay (Variables|Default|GetDelayOfReset))
  (bind _alpha (Timeline|Timeline_0 PlayFromStart)
    (:Update
      (Transformation|SetWorldRotation _sm_valve_01 (Math|Rotator|Lerp(Rotator) (Transformation|GetWorldRotation _sm_valve_01) (Math|Rotator|MakeRotator 24.0 (.pitch _returnvalue) (.yaw _returnvalue)) _alpha) false false)
      (Default|CallReactivateWater)
      (Utilities|FlowControl|RetriggerableDelay (Variables|Default|GetDelayBeforeReusable))
      (Variables|Default|SetIsActivated false))))

(event Custom|launchTestmovement
  (bind _sm_valve_01 (Variables|Default|GetSM_Valve_01))
  (bind _returnvalue (Transformation|GetWorldRotation _sm_valve_01))
  (Default|CallDesactivateWater)
  (Utilities|FlowControl|RetriggerableDelay (Variables|Default|GetDelayOfReset))
  (bind _alpha (Timeline|Timeline PlayFromStart)
    (:Update
      (Transformation|SetWorldRotation _sm_valve_01 (Math|Rotator|Lerp(Rotator) (Transformation|GetWorldRotation _sm_valve_01) (Math|Rotator|MakeRotator 24.0 (.pitch _returnvalue) (.yaw _returnvalue)) _alpha) false false)
      (Default|CallReactivateWater))))

(event EventTick
  (params (DeltaSeconds :type Float%20%28single-precision%29))
  (CallFunction|UpdateRotation))

(event EventBeginPlay
  (Utilities|FlowControl|Sequence
    (:then_0
      (bind _returnvalue (Actor|GetActorOfClass "/Game/Gameplay/WaterLevel/BP_PipeManager.BP_PipeManager_C"))
      (Variables|Default|SetPipeManagerRef _returnvalue)
      ;[1 1 1] Reset
      (EventDispatchers|BindEventtoDesactivateWater (delegate Custom|LaunchDelay))
      (EventDispatchers|BindEventtoTest2 (delegate Custom|launchTestmovement)))
    (:then_1
      (Audio|Components|Audio|Play (Variables|Default|GetMS_Valve) 0.0))))

(fn ConstructionScript)

(fn UpdateRotation
  (bind _sm_valve_01 (Variables|Default|GetSM_Valve_01))
  (if (not (Variables|Default|GetIsActivated))
    ;[1 1 1] V1
    (Utilities|IsValid (Variables|Default|GetMotion%20Controller)
      (:Is%20Valid
        ;[1 1 1] V2
        (bind _output_get (Variables|Default|SetCurentAngle (Math|Interpolation|FInterpTo (Variables|Default|GetCurentAngle) (* (Math|Rotator|NormalizeAxis (Math|Vector|DotProduct (Math|Rotator|GetRotationXVector (Math|Rotator|FindLookatRotation (Transformation|GetWorldLocation _sm_valve_01) (Transformation|GetWorldLocation (Variables|Default|GetMotion%20Controller)))) (Math|Vector|GetRightVector (Transformation|GetWorldRotation _sm_valve_01)))) 35.0) (Utilities|Time|GetWorldDeltaSeconds) 0.0)))
        (Transformation|AddLocalRotation (Variables|Default|GetSM_Valve_01) (Math|Rotator|MakeRotator _output_get 0.0 0.0) false false)
        (if (>= (.roll (Transformation|GetWorldRotation (Variables|Default|GetSM_Valve_01))) (Variables|Default|GetRotationValueDetection))
          (Default|CallDesactivateWater)
          (Variables|Default|SetIsActivated true))))))

(fn DesactivateWater
  (Class|AudioParameterControllerInterface|SetTriggerParameter (Variables|Default|GetMS_Valve) "PlayValveUse"))

(fn Test
  (Default|CallTest2))