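; Grabbable scotch tape for the water level that patches active BP_Leak actors when released on them.
; Grabbing reveals the meshes, and TapeCollision overlaps track the target leak and whether it can be fixed.
; Dropping on a valid leak deactivates and fixes it, then returns the tape hidden to its BeginPlay location.
; Otherwise the tape falls with physics until the Lifetime timeline finishes and triggers the same reset.
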(event OnGrabbed(GrabComponent)
  (Rendering|SetVisibility (Variables|Default|GetStaticMesh) true false))

(event OnDropped(GrabComponent)
  (bind _leaktofix (Variables|Default|GetLeakToFix))
  (bind _staticmesh (Variables|Default|GetStaticMesh))
  (if (Variables|Default|GetCanFix)
    (Utilities|IsValid _leaktofix
      (:Is%20Valid
        (Variables|/Game/Gameplay/WaterLevel/BP_Leak.BP_Leak_C|SetIsActive _leaktofix false)
        (Default|FixLeak _leaktofix)))
    (else
      (Physics|SetSimulatePhysics (Variables|Default|GetTape) true)
      ;[1 1 1] Reset position une fois laché
      (Timeline|lifetime Play
        (:Finished
          _))))
  (Transformation|SetWorldLocation (Variables|Default|GetTape) (Variables|Default|GetTapeLocation) false false)
  (Physics|SetSimulatePhysics _staticmesh false)
  (Rendering|SetVisibility _staticmesh false false))

(event OnComponentBeginOverlap(TapeCollision)
  (params (OverlappedComponent :type Primitive%20Component%20Object%20Reference) (OtherActor :type Actor%20Object%20Reference) (OtherComp :type Primitive%20Component%20Object%20Reference) (OtherBodyIndex :type Integer) (bFromSweep :type Boolean) (SweepResult :type Hit%20Result%20Structure%20%28by%20ref%29))
  (bind _asbp_leak (Utilities|Casting|CastToBP_Leak OtherActor))
  (if (Variables|/Game/Gameplay/WaterLevel/BP_Leak.BP_Leak_C|GetIsActive _asbp_leak)
    (Variables|Default|SetLeakToFix _asbp_leak)
    (Variables|Default|SetCanFix true)))

(event OnComponentEndOverlap(TapeCollision)
  (params (OverlappedComponent :type Primitive%20Component%20Object%20Reference) (OtherActor :type Actor%20Object%20Reference) (OtherComp :type Primitive%20Component%20Object%20Reference) (OtherBodyIndex :type Integer))
  (bind _asbp_leak (Utilities|Casting|CastToBP_Leak OtherActor))
  (if (Variables|/Game/Gameplay/WaterLevel/BP_Leak.BP_Leak_C|GetIsActive _asbp_leak)
    (Variables|Default|SetCanFix false)))

(event EventBeginPlay
  (Variables|Default|SetTapeLocation (Transformation|GetWorldLocation (Variables|Default|GetTape))))

(fn ConstructionScript)