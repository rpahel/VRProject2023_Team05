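; BP_Leak1 is a pipe leak actor that can be activated and fixed, with looks that follow the rising water level.
; While active, Tick compares GI_Water's WaterLevel to its height, showing a sphere when submerged or a leak mesh otherwise.
; The mesh's "In" morph target tracks the water within LeakHeight.
; Activation and fixing trigger MetaSound cues; fixing also decrements LeaksAmount and updates PipeManager's leak lists.
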(event EventBeginPlay
  ;[1 1 1] get game instance
  (bind _asgi_water (Utilities|Casting|CastToGI_Water (Game|GetGameInstance)))
  (Variables|Default|SetGameInstance _asgi_water)
  (Variables|Default|SetIsActive false))

(event EventTick
  (params (DeltaSeconds :type Float%20%28single-precision%29))
  (bind _returnvalue (Transformation|GetActorLocation))
  (bind _sphere (Variables|Default|GetSphere))
  (bind _gameinstance (Variables|Default|GetGameInstance))
  (bind _returnvalue_2 (Rendering|IsVisible _sphere))
  (bind _waterlevel (Variables|/Game/Gameplay/WaterLevel/GI_Water.GI_Water_C|GetWaterLevel _gameinstance))
  (if (Variables|Default|GetIsActive)
    ;[1 1 1] Check water level
    (if (> (Variables|/Game/Gameplay/WaterLevel/GI_Water.GI_Water_C|GetWaterLevel (Variables|Default|GetGameInstance)) (.z _returnvalue))
      ;[1 1 1] changement de modèle
      (if (not _returnvalue_2)
        (Rendering|SetVisibility (Variables|Default|GetSphere) true false)
        (Rendering|SetVisibility (Variables|Default|GetSM_Fuite_01) false false))
      (else
        (Utilities|FlowControl|Sequence
          (:then_0
            (if _returnvalue_2
              (Rendering|SetVisibility (Variables|Default|GetSM_Fuite_01) true false)
              (Rendering|SetVisibility (Variables|Default|GetSphere) false false)))
          (:then_1
            (if (> _waterlevel (- (.z _returnvalue) (Variables|Default|GetLeakHeight)))
              ;[1 1 1] Règle la hauteur du mesh
              (Components|SkeletalMesh|SetMorphTarget (Variables|Default|GetSM_Fuite_01) "In" (- 1.0 (/ (- (.z _returnvalue) _waterlevel) (Variables|Default|GetLeakHeight))) true))))))
    (elif (or (Rendering|IsVisible (Variables|Default|GetSphere)) (Rendering|IsVisible (Variables|Default|GetSM_Fuite_01)))
      (CallFunction|NotVisible))))

(fn ConstructionScript)

(fn ActivateLeak
  (bind _ms_water (Variables|Default|GetMS_Water))
  (Audio|Components|Audio|Play _ms_water 0.0)
  (Class|AudioParameterControllerInterface|SetTriggerParameter _ms_water "PlaySpray")
  (Variables|Default|SetIsActive true)
  (if (> (Variables|/Game/Gameplay/WaterLevel/GI_Water.GI_Water_C|GetWaterLevel (Variables|Default|GetGameInstance)) (.z (Transformation|GetActorLocation)))
    (Rendering|SetVisibility (Variables|Default|GetSphere) true false)
    (else
      (Rendering|SetVisibility (Variables|Default|GetSM_Fuite_01) true false))))

(fn FixLeak
  (bind _self self)
  (bind _ms_water (Variables|Default|GetMS_Water))
  (bind _pipemanager (Variables|Default|GetPipeManager))
  (bind _ms_scotch (Variables|Default|GetMS_Scotch))
  (Audio|Components|Audio|Play _ms_scotch 0.0)
  (Class|AudioParameterControllerInterface|SetTriggerParameter _ms_scotch "PlayScotch")
  (Audio|Components|Audio|Play _ms_water 0.0)
  (Class|AudioParameterControllerInterface|SetTriggerParameter _ms_water "StopSpray")
  (Math|Integer|DecrementInt (Variables|/Game/Gameplay/WaterLevel/GI_Water.GI_Water_C|GetLeaksAmount (Variables|Default|GetGameInstance))
    (:%20%20
      (Utilities|Array|Add (Variables|/Game/Gameplay/WaterLevel/BP_PipeManager.BP_PipeManager_C|GetLeaks _pipemanager) _self)
      (Utilities|Array|RemoveItem (Variables|/Game/Gameplay/WaterLevel/BP_PipeManager.BP_PipeManager_C|GetLeaks_Active _pipemanager) _self))))

(fn NotVisible
  (Rendering|SetVisibility (Variables|Default|GetSphere) false false)
  (Rendering|SetVisibility (Variables|Default|GetSM_Fuite_01) false false))

(fn VisibleAgain
  (if (> (Variables|/Game/Gameplay/WaterLevel/GI_Water.GI_Water_C|GetWaterLevel (Variables|Default|GetGameInstance)) (.z (Transformation|GetActorLocation)))
    (Rendering|SetVisibility (Variables|Default|GetSphere) true false)
    (else
      (Rendering|SetVisibility (Variables|Default|GetSM_Fuite_01) true false))))