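; BP_LilScotch is a grabbable tape prop for the water level that returns to its starting spot after being dropped.
; It caches the Tape component's world location at BeginPlay and makes it visible when the GrabComponent reports a grab, along with a debug print.
; Dropping it enables physics and starts the Lifetime timeline, whose completion restores the location (not rotation), disables physics and hides the tape.
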(event OnGrabbed(GrabComponent)
  (Development|PrintString "Hello")
  (Rendering|SetVisibility (Variables|Default|GetTape) true false))

(event OnDropped(GrabComponent)
  (bind _tape (Variables|Default|GetTape))
  (Physics|SetSimulatePhysics (Variables|Default|GetTape) true)
  (Timeline|lifetime PlayFromStart
    (:Finished
      (Transformation|SetWorldLocation (Variables|Default|GetTape) (Variables|Default|GetTapeLocation) false false)
      (Physics|SetSimulatePhysics _tape false)
      (Rendering|SetVisibility _tape false false))))

(event EventBeginPlay
  (Variables|Default|SetTapeLocation (Transformation|GetWorldLocation (Variables|Default|GetTape))))

(fn ConstructionScript)