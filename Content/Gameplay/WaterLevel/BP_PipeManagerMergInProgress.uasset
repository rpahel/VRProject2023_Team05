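; Pipe manager that spawns water leaks over time by activating pre-placed BP_Leak actors, tracking the count in GI_Water.
; A looping timer moves a random idle leak to the active list, up to a maximum; the re-randomized delay never resets the timer.
; BP_Valve events pause or resume spawning, toggling active leaks' state and visibility, plus BP_WaterLevel's rising flag when leaks are active.
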(event Custom|StopWater
  ;[1 1 1] Get Valve
  (CallFunction|StopLeaks))

(event Custom|NewLeak
  (bind _gameinstance (Variables|Default|GetGameInstance))
  (bind _leaks (Variables|Default|GetLeaks))
  (if (not (Math|Boolean|ORBoolean (Utilities|Array|IsEmpty (Variables|Default|GetLeaks)) (>= (Variables|/Game/Gameplay/WaterLevel/GI_Water.GI_Water_C|GetLeaksAmount (Variables|Default|GetGameInstance)) (Variables|Default|GetMaxLeaks)) (Variables|Default|GetStoppedLeaks)))
    ;[1 1 1] Nouvelle fuite toute les X sec
    (Development|PrintString "New leak :0")
    (Variables|Default|SetLeakDelay (Math|Random|RandomFloatinRange (Variables|Default|GetLeakDelayMin) (Variables|Default|GetLeakDelayMax)))
    (bind _result (Math|Integer|IncrementInt (Variables|/Game/Gameplay/WaterLevel/GI_Water.GI_Water_C|GetLeaksAmount _gameinstance))
      (:%20%20
        (Variables|/Game/Gameplay/WaterLevel/GI_Water.GI_Water_C|SetLeaksAmount _gameinstance _result)
        ;[1 1 1] Placement de la fuite
        (Variables|Default|SetItemToRemove (.OutIndex (Utilities|Array|Random _leaks)))
        (Default|ActivateLeak (Utilities|Array|Get(acopy) _leaks (Variables|Default|GetItemToRemove)))
        (Utilities|Array|Add (Variables|Default|GetLeaks_Active) (Utilities|Array|Get(acopy) _leaks (Variables|Default|GetItemToRemove)))
        (Utilities|Array|RemoveItem _leaks (Utilities|Array|Get(acopy) _leaks (Variables|Default|GetItemToRemove)))))))

(event Custom|EnableWater
  ;[1 1 1] Get Valve
  (CallFunction|EnableLeaks))

(event EventBeginPlay
  ;[1 1 1] get game instance
  (bind _asgi_water (Utilities|Casting|CastToGI_Water (Game|GetGameInstance)))
  (bind _output_get (Variables|Default|SetGameInstance _asgi_water))
  (Variables|/Game/Gameplay/WaterLevel/GI_Water.GI_Water_C|SetLeaksAmount _output_get 0)
  ;[1 1 1] Get Valve
  (bind _returnvalue (Actor|GetActorOfClass "/Game/Gameplay/WaterLevel/BP_Valve.BP_Valve_C"))
  (bind _output_get_2 (Variables|Default|SetValveRef _returnvalue))
  (EventDispatchers|BindEventtoDesactivateWater _output_get_2 (delegate Custom|StopWater))
  (EventDispatchers|BindEventtoReactivateWater _output_get_2 (delegate Custom|EnableWater))
  ;[1 1 1] get leaks
  (bind _outactors (Actor|GetAllActorswithInterface "/Game/Gameplay/WaterLevel/I_Leak.I_Leak_C"))
  (for _array_element _outactors
    (bind _asbp_leak (Utilities|Casting|CastToBP_Leak _array_element))
    (Variables|/Game/Gameplay/WaterLevel/BP_Leak.BP_Leak_C|SetPipeManager _asbp_leak self)
    (Utilities|Array|Add (Variables|Default|GetLeaks) _asbp_leak))
  ;[1 1 1] lance le timer des fuites
  (Utilities|Time|SetTimerbyFunctionName 0 "NewLeak" (Variables|Default|GetLeakDelay) true))

(event EventTick
  (params (DeltaSeconds :type Float%20%28single-precision%29)))

(fn ConstructionScript)

(fn StopLeaks
  (Variables|Default|SetStoppedLeaks true)
  (for _array_element (Variables|Default|GetLeaks_Active)
    (Variables|/Game/Gameplay/WaterLevel/BP_Leak.BP_Leak_C|SetIsActive _array_element false)
    (Default|NotVisible _array_element)
    (bind _returnvalue (Actor|GetActorOfClass "/Game/Gameplay/WaterLevel/BP_WaterLevel.BP_WaterLevel_C"))
    (Utilities|IsValid _returnvalue
      (:Is%20Valid
        (Variables|/Game/Gameplay/WaterLevel/BP_WaterLevel.BP_WaterLevel_C|SetWaterRising _returnvalue false)))))

(fn EnableLeaks
  (Variables|Default|SetStoppedLeaks false)
  (for _array_element (Variables|Default|GetLeaks_Active)
    (Variables|/Game/Gameplay/WaterLevel/BP_Leak.BP_Leak_C|SetIsActive _array_element true)
    (Default|VisibleAgain _array_element)
    (bind _returnvalue (Actor|GetActorOfClass "/Game/Gameplay/WaterLevel/BP_WaterLevel.BP_WaterLevel_C"))
    (Utilities|IsValid _returnvalue
      (:Is%20Valid
        (Variables|/Game/Gameplay/WaterLevel/BP_WaterLevel.BP_WaterLevel_C|SetWaterRising _returnvalue true)))))