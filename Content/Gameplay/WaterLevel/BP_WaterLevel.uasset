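; BP_WaterLevel is the rising water actor that triggers a game over when it climbs too high.
; On BeginPlay it caches the GI_Water game instance.
; While WaterRising is set, each Tick moves it up by a base speed times the instance's leak count, without delta-time scaling, and writes its Z back as WaterLevel.
; Each Tick also checks LoseHeight, showing W_LoseScreen and pausing once reached.
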(event EventTick
  (params (DeltaSeconds :type Float%20%28single-precision%29))
  (Utilities|FlowControl|Sequence
    (:then_0
      (if (Variables|Default|GetWaterRising)
        ;[1 1 1] augmentation niveau de l'eau
        (Transformation|AddActorLocalOffset (Math|Vector|MakeVector 0.0 0.0 (* (Variables|Default|GetBaseRisingSpeed) (Variables|/Game/Gameplay/WaterLevel/GI_Water.GI_Water_C|GetLeaksAmount (Variables|Default|GetGame%20Instance)))) false false)
        (Variables|/Game/Gameplay/WaterLevel/GI_Water.GI_Water_C|SetWaterLevel (Variables|Default|GetGame%20Instance) (.z (Transformation|GetActorLocation)))))
    (:then_1
      (if (>= (.z (Transformation|GetActorLocation)) (Variables|Default|GetLoseHeight))
        (bind _returnvalue (UserInterface|CreateWidget "/Game/Gameplay/WaterLevel/W_LoseScreen.W_LoseScreen_C"))
        (UserInterface|Viewport|AddtoViewport _returnvalue 0)
        (Game|SetGamePaused true)))))

(event EventBeginPlay
  ;[1 1 1] get game instance
  (bind _asgi_water (Utilities|Casting|CastToGI_Water (Game|GetGameInstance)))
  (Variables|Default|SetGame%20Instance _asgi_water))

(fn ConstructionScript)