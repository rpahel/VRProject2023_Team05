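; Pipe manager for the water level that periodically springs leaks in the level's pipes, up to a maximum count.
; On BeginPlay it resets the GI_Water leak count, registers itself with each BP_Leak found through I_Leak, and starts a looping timer.
; Each tick of that timer below the cap activates a random leak, increments the count and updates the inactive and active lists.
; LeakDelay is re-randomized, but the running timer is never reset.
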(event Custom|NewLeak
  (bind _gameinstance (Variables|Default|GetGameInstance))
  (bind _leaks (Variables|Default|GetLeaks))
  (if (not (or (Utilities|Array|IsEmpty (Variables|Default|GetLeaks)) (>= (Variables|/Game/Gameplay/WaterLevel/GI_Water.GI_Water_C|GetLeaksAmount (Variables|Default|GetGameInstance)) (Variables|Default|GetMaxLeaks))))
    ;[1 1 1] Nouvelle fuite toute les X sec
    (Development|PrintString "New leak :0")
    (Variables|Default|SetLeakDelay (Math|Random|RandomFloatinRange (Variables|Default|GetLeakDelayMin) (Variables|Default|GetLeakDelayMax)))
    (bind _result (Math|Integer|IncrementInt (Variables|/Game/Gameplay/WaterLevel/GI_Water.GI_Water_C|GetLeaksAmount _gameinstance))
      (:%20%20
        (Variables|/Game/Gameplay/WaterLevel/GI_Water.GI_Water_C|SetLeaksAmount _gameinstance _result)
        ;[1 1 1] Placement de la fuite
        (Variables|Default|SetItemToRemove (.OutIndex (Utilities|Array|Random _leaks)))
        (Default|ActivateLeak (Utilities|Array|Get(acopy) _leaks (Variables|Default|GetItemToRemove)))
        (Utilities|Array|RemoveItem _leaks (Utilities|Array|Get(acopy) _leaks (Variables|Default|GetItemToRemove)))
        (Utilities|Array|Add (Variables|Default|GetLeaks_Active) (Utilities|Array|Get(acopy) _leaks (Variables|Default|GetItemToRemove)))))))

(event EventBeginPlay
  ;[1 1 1] get game instance
  (bind _asgi_water (Utilities|Casting|CastToGI_Water (Game|GetGameInstance)))
  (bind _output_get (Variables|Default|SetGameInstance _asgi_water))
  (Variables|/Game/Gameplay/WaterLevel/GI_Water.GI_Water_C|SetLeaksAmount _output_get 0)
  ;[1 1 1] get leaks
  (bind _outactors (Actor|GetAllActorswithInterface "/Game/Gameplay/WaterLevel/I_Leak.I_Leak_C"))
  (for _array_element _outactors
    (bind _asbp_leak (Utilities|Casting|CastToBP_Leak _array_element))
    (Variables|/Game/Gameplay/WaterLevel/BP_Leak.BP_Leak_C|SetPipeManager _asbp_leak self)
    (Utilities|Array|Add (Variables|Default|GetLeaks) _asbp_leak))
  ;[1 1 1] lance le timer des fuites
  (Utilities|Time|SetTimerbyFunctionName 0 "NewLeak" (Variables|Default|GetLeakDelay) true))

(event EventTick
  (params (DeltaSeconds :type Float%20%28single-precision%29)))

(fn ConstructionScript)