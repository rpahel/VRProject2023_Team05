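; BP_SubLight is a light that turns on and off when a cable is plugged into or unplugged from its referenced ElectricBox.
; It binds to the box's plug events on BeginPlay, printing an error if the reference is missing.
; A matching plug index switches point light intensity and mesh material.
; MSLight, likely a MetaSound, receives on/off triggers for any plug index, since that call sits outside the index check.
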(event Custom|OnCablePlugged
  (params (FemalePlugIndex :type Integer))
  ;[1 1 1] Bind plugged
  (CallFunction|CablePlugged FemalePlugIndex)
  (Class|AudioParameterControllerInterface|SetTriggerParameter (Variables|Default|GetMS_Light) "LightOn"))

(event Custom|OnCableUnplugged
  (params (FemalePlugIndex :type Integer))
  ;[1 1 1] Bind Unplugged
  (CallFunction|CableUnplugged FemalePlugIndex)
  (Class|AudioParameterControllerInterface|SetTriggerParameter (Variables|Default|GetMS_Light) "LightOff"))

(event EventBeginPlay
  (bind _electricbox (Variables|SubLight|GetElectricBox))
  (Utilities|IsValid _electricbox
    (:Is%20Valid
      ;[1 1 1] Bind plugged
      (EventDispatchers|BindEventtoOnCablePlugged _electricbox (delegate Custom|OnCablePlugged))
      ;[1 1 1] Bind Unplugged
      (EventDispatchers|BindEventtoOnCableUnplugged _electricbox (delegate Custom|OnCableUnplugged)))
    (:Is%20Not%20Valid
      (Development|PrintString "Sublight ne connait pas ElectricBox dont elle dépend. Oublie de référencement ?" true true "(R=1.000000,G=0.000000,B=0.000000,A=1.000000)" 1e+02))))

(fn ConstructionScript)

(fn CablePlugged
  (params (PlugIndex :type Integer))
  (bind _pointlight (Variables|Default|GetPointLight))
  (bind _sublight_sm (Variables|Default|GetSubLight_SM))
  (if (== (Variables|SubLight|GetFemalePlugIndex) PlugIndex)
    ;[1 1 1] Intensité lumière
    (Utilities|IsValid _pointlight
      (:Is%20Valid
        (Rendering|Components|Light|SetIntensity _pointlight (Variables|Appearance|GetLightIntensityOn))
        ;[1 1 1] Set Material
        (Utilities|IsValid _sublight_sm
          (:Is%20Valid
            (Rendering|Material|SetMaterial _sublight_sm 0 (Variables|Appearance|GetSublightMaterialLit))))))))

(fn CableUnplugged
  (params (PlugIndex :type Integer))
  (bind _pointlight (Variables|Default|GetPointLight))
  (bind _sublight_sm (Variables|Default|GetSubLight_SM))
  (if (== (Variables|SubLight|GetFemalePlugIndex) PlugIndex)
    ;[1 1 1] Intensité lumière
    (Utilities|IsValid _pointlight
      (:Is%20Valid
        (Rendering|Components|Light|SetIntensity _pointlight 0.0)
        ;[1 1 1] Set Material
        (Utilities|IsValid _sublight_sm
          (:Is%20Valid
            (Rendering|Material|SetMaterial _sublight_sm 0 (Variables|Appearance|GetSublightMaterialUnlit))))))))

(fn TestLighton
  (CallFunction|OnCablePlugged))

(fn TestLightOff
  (CallFunction|CableUnplugged))